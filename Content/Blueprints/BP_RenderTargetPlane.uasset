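; BP_RenderTargetPlane is a plane actor that displays its own render target, which can be filled by a solid color shader.
; The construction script creates the render target from size, format and clear color variables, then binds it to a dynamic M_RenderTargetPlane material on the plane.
; ApplyShader passes that target and ShadingColor to RenderSolidColorShader; nothing in this Blueprint calls it, as the event graph is empty.
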(fn `ApplyShader`
  (`MeshPainterFunctionLibrary.RenderSolidColorShader` (`self.RenderTarget`) (`self.ShadingColor`)))

(fn `UserConstructionScript`
  (bind _returnvalue (`PrimitiveComponent.CreateDynamicMaterialInstance` (`self.Plane`) 0 "/Game/Materials/M_RenderTargetPlane.M_RenderTargetPlane" "None"))
  (bind _returnvalue_2 (`KismetRenderingLibrary.CreateRenderTarget2D` (`self.RenderTargetWidth`) (`self.RenderTargetHeight`) (`self.RenderTargetFormat`) (`self.RenderTargetColor`) true))
  (bind _output_get (set `self.RenderTarget` _returnvalue_2))
  (`MaterialInstanceDynamic.SetTextureParameterValue` _returnvalue "RenderTarget" _output_get))